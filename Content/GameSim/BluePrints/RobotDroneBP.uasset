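; Robot drone actor that wanders on its own using a Tick-driven state machine and captures screenshots as it goes.
; A forward line trace chooses between stepping forward and, when an obstacle is within CollideDistance, yawing one degree.
; Each move leads to a delay that triggers screenshot, camera-view actor query and next-sequence calls before tracing again.
; GetRandomRotation uses a time-seeded stream but is never called, and DropSpecialItem is empty.
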(event EventBeginPlay
  ;[1 0.4937 0.944 1 32] Begin - SET RANDOM SEED
  (bind _output_get (Variables|Default|SetCurrentDate (Math|DateTime|UTCNow)))
  (Math|Random|SetRandomStreamSeed (Variables|Default|GetRandomStream) (Math|DateTime|GetMillisecond _output_get)))

(event Collision|EventActorBeginOverlap
  (params (OtherActor :type Actor%20Object%20Reference))
  (Development|PrintString (Utilities|GetDisplayName OtherActor) true true "(R=1.000000,G=0.000000,B=0.000000,A=1.000000)"))

(event EventTick
  (params (DeltaSeconds :type Float%20%28single-precision%29))
  (bind _robotbody (Variables|Default|GetRobotBody))
  (bind _robotbody_2 (Variables|Default|GetRobotBody))
  (bind _robotbody_3 (Variables|Default|GetRobotBody))
  (bind _returnvalue (Transformation|GetWorldRotation _robotbody))
  (bind _returnvalue_2 (Transformation|GetWorldRotation _robotbody_2))
  (bind _returnvalue_3 (Transformation|GetWorldLocation _robotbody_2))
  (bind _returnvalue_4 (Math|Vector|GetForwardVector _returnvalue_2))
  (bind _returnvalue_5 (* _returnvalue_4 1.0))
  (bind _returnvalue_6 (+ _returnvalue_3 _returnvalue_5))
  ;[0.4635 0.005974 0.3426 1 32] Event Tick - SWITCH
  (switch Utilities|FlowControl|Switch|SwitchonPawnStates (Variables|Default|GetCurrentState)
    (:NewEnumerator4
      ;[1 0.2154 0.2851 1 32] LINE TRACE
      (bind (_outhit _returnvalue_7) (Collision|LineTraceByChannel _returnvalue_6 (+ _returnvalue_6 (* _returnvalue_4 2e+02)) "TraceTypeQuery1" false 0 "ForDuration" true "(R=0.000000,G=0.822435,B=1.000000,A=1.000000)" "(R=0.000000,G=1.000000,B=0.000000,A=1.000000)" 1.0))
      (if _returnvalue_7
        (bind _output_get (Variables|Default|SetDistanceToObj (.Distance (Collision|BreakHitResult _outhit))))
        (if (< _output_get (Variables|Default|GetCollideDistance))
          (Variables|Default|SetCurrentState "NewEnumerator2")
          (else
            (Variables|Default|SetCurrentState "NewEnumerator1" :!label _label)))
        (else
          (goto _label)))
      (Development|PrintString (Utilities|String|ToString(Float) _output_get) true true "(R=0.869792,G=0.000000,B=0.733969,A=1.000000)"))
    (:NewEnumerator1
      ;[0.3797 1 0.577 1 32] MOVE FORWARD
      (Transformation|SetWorldLocation _robotbody_3 (+ (Transformation|GetWorldLocation _robotbody_3) (* (Math|Vector|GetForwardVector _robotbody_3) 1e+01)) false false)
      (Variables|Default|SetCurrentState "NewEnumerator5"))
    (:NewEnumerator2
      ;[0 0.3233 1 1 32] RANDOM ROTATE
      (Transformation|SetWorldRotation _robotbody (Math|Rotator|MakeRotator (.roll _returnvalue) (.pitch _returnvalue) (+ (.yaw _returnvalue) 1.0)) false false)
      (Variables|Default|SetCurrentState "NewEnumerator5"))
    (:NewEnumerator5
      ;[1 0.9791 0.121 1 32] WAIT
      (Utilities|FlowControl|Delay (Variables|Default|GetWaitTime))
      (Class|RobotDrone|TakeScreenShot)
      (Class|RobotDrone|GetAllActorsinCameraView 1.0)
      (Class|RobotDrone|StartNextSequence)
      (CallFunction|DropSpecialItem)
      (Variables|Default|SetCurrentState "NewEnumerator4"))))

(fn ConstructionScript)

(fn GetRandomRotation
  (params (RangeLow :type Float%20%28single-precision%29) (RangeHigh :type Float%20%28single-precision%29))
  (bind _randomstream (Variables|Default|GetRandomStream))
  (Variables|Default|SetRotResult (Math|Random|RandomFloatinRangefromStream RangeLow RangeHigh _randomstream))
  (if (> (Math|Random|RandomIntegerinRangefromStream 0 100 _randomstream) 50)
    (Variables|Default|SetRotResult (* (Variables|Default|GetRotResult) -1.0)))
  (return (Variables|Default|GetRotResult)))

(fn DropSpecialItem)